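; Side-scrolling camera actor that becomes the player's view target on BeginPlay and follows ActorToFollow in X and Z.
; The construction script places it at the followed actor's X with a Y offset and a fixed or offset height, then yaws it toward that actor.
; Each tick, dead-zone functions move it only when the actor leaves the margins, with FixedZValue overriding height while the actor is below it.
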(event `self.ReceiveBeginPlay`
  (`PlayerController.SetViewTargetWithBlend` (`GameplayStatics.GetPlayerController` 0) self 0.0 "VTBlend_Linear" 0.0 false))

(event `self.ReceiveTick`
  (params (DeltaSeconds :type "Float (single-precision)"))
  (bind _camx (`self.GetNewXValue`))
  (bind _output_get (set `self.CameraX` _camx))
  (bind _camz (`self.GetNewZValue`))
  (bind _output_get_2 (set `self.CameraZ` _camz))
  (`self.K2_SetActorLocation` (`KismetMathLibrary.MakeVector` _output_get 0.0 _output_get_2)))

(fn `GetNewXValue`
  (returns (CamX :type "Float (double-precision)"))
  (bind _returnvalue_x (`KismetMathLibrary.BreakVector` (`self.K2_GetActorLocation`)))
  (bind _returnvalue_x_2 (`KismetMathLibrary.BreakVector` (`self.K2_GetActorLocation`)))
  (bind _returnvalue_x_3 (`KismetMathLibrary.BreakVector` (`self.K2_GetActorLocation` (`self.ActorToFollow`))))
  (bind _returnvalue_x_4 (`KismetMathLibrary.BreakVector` (`self.K2_GetActorLocation` (`self.ActorToFollow`))))
  (bind _returnvalue (- _returnvalue_x_4 (`self.XDeadZone`)))
  (bind _returnvalue_2 (+ _returnvalue_x_3 (`self.XDeadZone`)))
  (if (> _returnvalue _returnvalue_x_2)
    (return _returnvalue)
    (elif (< _returnvalue_2 _returnvalue_x)
      (return _returnvalue_2)
      (else
        (return (`self.CameraX`))))))

(fn `GetNewZValue`
  (returns (CamZ :type "Float (double-precision)"))
  (bind (_returnvalue_x _returnvalue_y _returnvalue_z) (`KismetMathLibrary.BreakVector` (`self.K2_GetActorLocation`)))
  (bind (_returnvalue_x_2 _returnvalue_y_2 _returnvalue_z_2) (`KismetMathLibrary.BreakVector` (`self.K2_GetActorLocation`)))
  (bind (_returnvalue_x_3 _returnvalue_y_3 _returnvalue_z_3) (`KismetMathLibrary.BreakVector` (`self.K2_GetActorLocation` (`self.ActorToFollow`))))
  (bind (_returnvalue_x_4 _returnvalue_y_4 _returnvalue_z_4) (`KismetMathLibrary.BreakVector` (`self.K2_GetActorLocation` (`self.ActorToFollow`))))
  (bind (_returnvalue_x_5 _returnvalue_y_5 _returnvalue_z_5) (`KismetMathLibrary.BreakVector` (`self.K2_GetActorLocation` (`self.ActorToFollow`))))
  (bind _returnvalue (- _returnvalue_z_3 (`self.ZDeadZone`)))
  (bind _returnvalue_2 (+ _returnvalue_z_5 (`self.ZDeadZone`)))
  (if (> (`self.Fixed ZValue`) _returnvalue_z_4)
    (return (`self.Fixed ZValue`))
    (elif (> _returnvalue _returnvalue_z_2)
      (return _returnvalue)
      (elif (< _returnvalue_2 _returnvalue_z)
        (return _returnvalue_2)
        (else
          (return _returnvalue_z))))))

(fn `UserConstructionScript`
  (bind _actortofollow (`self.ActorToFollow`))
  (bind (_returnvalue_x _returnvalue_y _returnvalue_z) (`KismetMathLibrary.BreakVector` (`self.K2_GetActorLocation` _actortofollow)))
  (bind (_returnvalue_roll _returnvalue_pitch _returnvalue_yaw) (`KismetMathLibrary.BreakRotator` (`KismetMathLibrary.FindLookAtRotation` (`self.K2_GetActorLocation`) (`self.K2_GetActorLocation` (`self.ActorToFollow`)))))
  (`/Engine/EditorBlueprintResources/StandardMacros.IsValid` _actortofollow
    (:`Is Valid`
      (set `self.CameraX` _returnvalue_x)
      (if (!= (`self.Fixed ZValue`) 0.0)
        (set `self.CameraZ` (`self.Fixed ZValue`))
        (else
          (bind _output_get (set `self.CameraZ` (+ _returnvalue_z (`self.ZDeadZone`))))))
      (`self.K2_SetActorLocation` (`KismetMathLibrary.MakeVector` _returnvalue_x (`self.YOffset`) _output_get))
      (`self.K2_SetActorRotation` (`KismetMathLibrary.MakeRotator` 0.0 0.0 _returnvalue_yaw)))))