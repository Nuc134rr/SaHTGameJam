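; Game instance that drives level progression through a narrative sequence of stages of grief, from Intro through Denial, Anger, Bargaining, Depression and Acceptance.
; It keeps a persistent Level index across map loads.
; The overlappingtrigger event increments that index and opens the matching level by name from a fixed, ordered list.
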(event `overlappingtrigger`
  (bind _output_get (set `self.Level` (+ (`self.Level`) 1)))
  (`GameplayStatics.OpenLevel` (`|GetArrayItem` (`|MakeArray` (`self.Intro`) (`self.Denial`) (`self.Anger`) (`self.Bargaining`) (`self.Depression`) (`self.Acceptance`)) _output_get) false))