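; Clickable apple paper item from the Denial item set that the player picks up and carries.
; Clicking its paper sprite marks it collected and prints a debug message, provided the referenced Denial object's FirstConversation flag is false.
; Once collected, Tick snaps it to the Puddle pawn's sprite each frame, subtracting or adding a grab offset based on whether Puddle is moving right.
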(event `self.ReceiveTick`
  (params (DeltaSeconds :type "Float (single-precision)"))
  (bind _actorgraboffset (`self.actorGrabOffset`))
  ;[1 1 1] Apple Follows
  (if (`self.Collected`)
    (bind _aspuddle (cast `/Game/realDiles/Characters/Puddle/Puddle` (`GameplayStatics.GetPlayerPawn` 0)))
    (if true
      (if (`/Game/realDiles/Characters/Puddle/Puddle.bIsMovingRight` _aspuddle)
        (bind _returnvalue (`SceneComponent.K2_GetComponentLocation` (`PaperCharacter.Sprite` _aspuddle)))
        (`self.K2_SetActorLocation` (- _returnvalue _actorgraboffset))
        (else
          (`self.K2_SetActorLocation` (+ _returnvalue _actorgraboffset)))))))

(event `self.PaperSprite.OnClicked`
  (params (TouchedComponent :type "PrimitiveComponent Object Reference") (ButtonPressed :type "Key Structure"))
  ;[1 1 1] Item is collected
  (bind _asdenial (cast `/Game/realDiles/Characters/Denial/Denial` (`self.Denial`)))
  (if (not (`/Game/realDiles/Characters/Denial/Denial.First Conversation` _asdenial))
    (set `self.Collected` true)
    (`KismetSystemLibrary.PrintString` "Hello")))

(fn `UserConstructionScript`)