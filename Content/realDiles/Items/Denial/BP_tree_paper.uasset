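; Clickable paper tree item for Denial that drops its target paper apple.
; On click, if Denial's FirstConversation flag is false, a one-shot LeavesClicked guard lets it move the apple 350 units down in a single instant step.
; Pickup, follow-player, drop and stick-removal logic is left disconnected, so Tick, BeginDrop and RemoveStick do nothing.
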(event `self.Tree.OnClicked`
  (params (TouchedComponent :type "PrimitiveComponent Object Reference") (ButtonPressed :type "Key Structure"))
  (bind _targetapple (`self.TargetApple`))
  (bind (_returnvalue_x _returnvalue_y _returnvalue_z) (`KismetMathLibrary.BreakVector` (`self.K2_GetActorLocation` _targetapple)))
  ;[1 1 1] Drop the stick when the leaves are clicked
  (bind _asdenial (cast `/Game/realDiles/Characters/Denial/Denial` (`self.Denial`)))
  (if (`/Game/realDiles/Characters/Denial/Denial.First Conversation` _asdenial)
    _
    (elif (not (`self.bLeavesClicked`))
      (set `self.bLeavesClicked` true)
      (bind _asbp_apple_paper (cast `/Game/realDiles/Items/Denial/BP_apple_paper` _targetapple))
      (`self.K2_SetActorLocation` _asbp_apple_paper (`KismetMathLibrary.MakeVector` _returnvalue_x 0.0 (- _returnvalue_z 350.0)) false false)
      (`KismetSystemLibrary.PrintString` "tree"))))

(event `self.ReceiveTick`
  (params (DeltaSeconds :type "Float (single-precision)"))
  ;[1 1 1] Follow player according to direction
)

(fn `Begin Drop`
  (`|ExecutionSequence`
    (:`then_1`
      (return))))

(fn `Remove Stick`
  (return))

(fn `UserConstructionScript`)