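; BP_Cup is a clickable pickup that the Puddle player carries and that can appear filled with water.
; Clicking it sets the cup as clicked and flags Puddle as holding an item.
; While held, Tick teleports it beside Puddle's sprite by facing direction, and swaps its sprite and IsFull state from the river and waterfall flags.
; ChangeCupToFull has no effect, as its body never runs.
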(event `self.Cup.OnClicked`
  (params (TouchedComponent :type "PrimitiveComponent Object Reference") (ButtonPressed :type "Key Structure"))
  ;[1 1 1] Update Variables
  (if (not (`self.bIsClicked`))
    (set `self.bIsClicked` true)
    (bind _aspuddle (cast `/Game/realFiles/Characters/Puddle/Puddle` (`GameplayStatics.GetPlayerPawn` 0)))
    (set `/Game/realFiles/Characters/Puddle/Puddle.bDoesHaveItem` true _aspuddle)))

(event `self.ReceiveTick`
  (params (DeltaSeconds :type "Float (single-precision)"))
  (bind _actorgraboffset (`self.actorGrabOffset`))
  ;[1 1 1] Follow player according to direction
  (bind _aspuddle (cast `/Game/realFiles/Characters/Puddle/Puddle` (`GameplayStatics.GetPlayerPawn` 0)))
  (if (`self.bIsClicked`)
    (if (`/Game/realFiles/Characters/Puddle/Puddle.bIsMovingRight` _aspuddle)
      (bind _returnvalue (`SceneComponent.K2_GetComponentLocation` (`PaperCharacter.Sprite` _aspuddle)))
      (`SceneComponent.K2_SetWorldLocation` (`self.Cup`) (- _returnvalue _actorgraboffset) false true)
      (else
        (`SceneComponent.K2_SetWorldLocation` (`self.Cup`) (+ _returnvalue _actorgraboffset) false true)))
    (if (`self.IsCupFullRiver`)
      (`PaperSpriteComponent.SetSprite` (`self.Cup`) "/Game/realFiles/Items/Depression/cup_2_Sprite.cup_2_Sprite")
      (set `self.IsFull` true)
      (elif (`self.IsCupFullWaterFall`)
        (`PaperSpriteComponent.SetSprite` (`self.Cup`) "/Game/realFiles/Items/Depression/cup_2_Sprite.cup_2_Sprite")
        (set `self.IsFull` true)
        (else
          (`PaperSpriteComponent.SetSprite` (`self.Cup`) "/Game/realFiles/Items/Depression/cup_1_Sprite.cup_1_Sprite")
          (set `self.IsFull` false))))))

(fn `Change Cup To Full`
  (bind _cup (`self.Cup`))
  (cast `/Game/realFiles/Characters/Puddle/Puddle` (`GameplayStatics.GetPlayerPawn` 0))
  (while false
    (`SceneComponent.SetVisibility` _cup false false)
    (`PrimitiveComponent.SetCollisionEnabled` _cup "NoCollision")
    (set `self.bIsClicked` false))
  (return))

(fn `UserConstructionScript`)