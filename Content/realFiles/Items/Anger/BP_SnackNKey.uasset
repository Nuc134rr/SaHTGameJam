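; BP_SnackNKey is a carried snack item that turns into a key for the Puddle player.
; While Collected is set, Tick teleports both Snacky and Key to the player's sprite, flipping the grab offset by facing direction.
; Each of those ticks also runs RemoveSnack, which responds to KeyholeClicked by hiding the snack, disabling its collision and revealing the key.
; It then clears that flag and sets DoesHaveItem on Puddle.
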(event `self.ReceiveTick`
  (params (DeltaSeconds :type "Float (single-precision)"))
  (bind _actorgraboffset (`self.actorGrabOffset`))
  (if (`self.Collected`)
    (`self.Remove Snack`)
    (bind _aspuddle (cast `/Game/realFiles/Characters/Puddle/Puddle` (`GameplayStatics.GetPlayerPawn` 0)))
    (if (`/Game/realFiles/Characters/Puddle/Puddle.bIsMovingRight` _aspuddle)
      (bind _returnvalue (`SceneComponent.K2_GetComponentLocation` (`PaperCharacter.Sprite` _aspuddle)))
      (`SceneComponent.K2_SetWorldLocation` (`self.Snacky`) (- _returnvalue _actorgraboffset) false true)
      (`SceneComponent.K2_SetWorldLocation` (`self.Key`) (- _returnvalue _actorgraboffset) false true)
      (else
        (`SceneComponent.K2_SetWorldLocation` (`self.Snacky`) (+ _returnvalue _actorgraboffset) false true)
        (`SceneComponent.K2_SetWorldLocation` (`self.Key`) (+ _returnvalue _actorgraboffset) false true)))))

(fn `Remove Snack`
  (bind _snacky (`self.Snacky`))
  (bind _aspuddle (cast `/Game/realFiles/Characters/Puddle/Puddle` (`GameplayStatics.GetPlayerPawn` 0)))
  (while (`/Game/realFiles/Characters/Puddle/Puddle.bKeyholeClicked` _aspuddle)
    (`SceneComponent.SetVisibility` _snacky false false)
    (`PrimitiveComponent.SetCollisionEnabled` _snacky "NoCollision")
    (`SceneComponent.SetVisibility` (`self.Key`) true false)
    (bind _aspuddle_2 (cast `/Game/realFiles/Characters/Puddle/Puddle` (`GameplayStatics.GetPlayerPawn` 0)))
    (set `/Game/realFiles/Characters/Puddle/Puddle.bKeyholeClicked` false _aspuddle_2)
    (set `/Game/realFiles/Characters/Puddle/Puddle.bDoesHaveItem` true _aspuddle_2))
  (return))

(fn `UserConstructionScript`)