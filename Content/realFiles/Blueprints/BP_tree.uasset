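; Clickable tree puzzle prop that drops an item (the Apple component) for the player's Puddle pawn to collect.
; Once Denial's FirstConversation flag is false, clicking the tree lowers the Apple and disables tree collision.
; Clicking the Apple flags Puddle as holding an item, and Tick teleports it beside Puddle's sprite by movement direction.
; Tick also hides it when Puddle clicks the keyhole, resetting the click flags, or finishes the level.
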(event `self.Tree.OnClicked`
  (params (TouchedComponent :type "PrimitiveComponent Object Reference") (ButtonPressed :type "Key Structure"))
  ;[1 1 1] Drop the stick when the leaves are clicked
  (bind _asdenial (cast `/Game/realFiles/Characters/Denial/Denial` (`self.Denial`)))
  (if (`/Game/realFiles/Characters/Denial/Denial.First Conversation` _asdenial)
    _
    (elif (not (`self.bTreeClicked`))
      (set `self.bTreeClicked` true)
      (`self.Begin Drop`))))

(event `self.Apple.OnClicked`
  (params (TouchedComponent :type "PrimitiveComponent Object Reference") (ButtonPressed :type "Key Structure"))
  ;[1 1 1] Update Variables
  (if (not (`self.bIsClicked`))
    (set `self.bIsClicked` true)
    (bind _aspuddle (cast `/Game/realFiles/Characters/Puddle/Puddle` (`GameplayStatics.GetPlayerPawn` 0)))
    (set `/Game/realFiles/Characters/Puddle/Puddle.bDoesHaveItem` true _aspuddle)))

(event `self.ReceiveTick`
  (params (DeltaSeconds :type "Float (single-precision)"))
  (bind _actorgraboffset (`self.actorGrabOffset`))
  ;[1 1 1] Follow player according to direction
  (if (`self.bTreeClicked`)
    (`self.Remove Apple`)
    (bind _aspuddle (cast `/Game/realFiles/Characters/Puddle/Puddle` (`GameplayStatics.GetPlayerPawn` 0)))
    (if (`/Game/realFiles/Characters/Puddle/Puddle.FinishedLevel` _aspuddle)
      (`SceneComponent.SetVisibility` (`self.Apple`) false false)
      (elif (`self.bIsClicked`)
        (if (`/Game/realFiles/Characters/Puddle/Puddle.bIsMovingRight` _aspuddle)
          (bind _returnvalue (`SceneComponent.K2_GetComponentLocation` (`PaperCharacter.Sprite` _aspuddle)))
          (`SceneComponent.K2_SetWorldLocation` (`self.Apple`) (- _returnvalue _actorgraboffset) false true)
          (else
            (`SceneComponent.K2_SetWorldLocation` (`self.Apple`) (+ _returnvalue _actorgraboffset) false true)))))))

(fn `Begin Drop`
  (bind _apple (`self.Apple`))
  (`|ExecutionSequence`
    (:`then_0`
      (`SceneComponent.K2_SetWorldLocation` _apple (- (`SceneComponent.K2_GetComponentLocation` _apple) (0.0 0.0 400.0)) false false)
      (`PrimitiveComponent.SetCollisionEnabled` (`self.Tree`) "NoCollision"))
    (:`then_1`
      (return))))

(fn `Remove Apple`
  (bind _apple (`self.Apple`))
  (bind _aspuddle (cast `/Game/realFiles/Characters/Puddle/Puddle` (`GameplayStatics.GetPlayerPawn` 0)))
  (while (`/Game/realFiles/Characters/Puddle/Puddle.bKeyholeClicked` _aspuddle)
    (`SceneComponent.SetVisibility` _apple false false)
    (`PrimitiveComponent.SetCollisionEnabled` _apple "NoCollision")
    (bind _aspuddle_2 (cast `/Game/realFiles/Characters/Puddle/Puddle` (`GameplayStatics.GetPlayerPawn` 0)))
    (set `/Game/realFiles/Characters/Puddle/Puddle.bKeyholeClicked` false _aspuddle_2)
    (set `self.bIsClicked` false)
    (set `self.bTreeClicked` false))
  (return))

(fn `UserConstructionScript`)