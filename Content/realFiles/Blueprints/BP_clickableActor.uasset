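; A clickable item actor that the 2D side-scroller player picks up by clicking its Cube component.
; The first click sets IsClicked, increments the character's ItemCount and flags DoesHaveItem.
; While clicked, Tick teleports the Cube to the character sprite's location, offset by ActorGrabOffset to one side or the other according to IsMovingRight, so it follows the player.
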(event `self.Cube.OnClicked`
  (params (TouchedComponent :type "PrimitiveComponent Object Reference") (ButtonPressed :type "Key Structure"))
  ;[1 1 1] onClick
  (if (not (`self.bIsClicked`))
    (set `self.bIsClicked` true)
    (bind _as2dside_scroller_character (cast `/Game/realFiles/Blueprints/2DSideScrollerCharacter` (`GameplayStatics.GetPlayerPawn` 0)))
    (set `/Game/realFiles/Blueprints/2DSideScrollerCharacter.itemCount` (+ (`/Game/realFiles/Blueprints/2DSideScrollerCharacter.itemCount` _as2dside_scroller_character) 1) _as2dside_scroller_character)
    (set `/Game/realFiles/Blueprints/2DSideScrollerCharacter.bDoesHaveItem` true _as2dside_scroller_character)))

(event `self.ReceiveTick`
  (params (DeltaSeconds :type "Float (single-precision)"))
  (bind _actorgraboffset (`self.actorGrabOffset`))
  (if (`self.bIsClicked`)
    (bind _as2dside_scroller_character (cast `/Game/realFiles/Blueprints/2DSideScrollerCharacter` (`GameplayStatics.GetPlayerPawn` 0)))
    (if (`/Game/realFiles/Blueprints/2DSideScrollerCharacter.bIsMovingRight` _as2dside_scroller_character)
      (bind _returnvalue (`SceneComponent.K2_GetComponentLocation` (`PaperCharacter.Sprite` _as2dside_scroller_character)))
      (`SceneComponent.K2_SetWorldLocation` (`self.Cube`) (- _returnvalue _actorgraboffset) false true)
      (else
        (`SceneComponent.K2_SetWorldLocation` (`self.Cube`) (+ _returnvalue _actorgraboffset) false true)))))

(fn `UserConstructionScript`)