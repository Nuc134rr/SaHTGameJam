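; Game instance that tracks level progression through an intro and the five stages of grief.
; NewLevel prints a debug string, increments the stored Level index and opens the matching map by name from a hard-coded ordered array, with no bounds check.
; An unconnected branch that would trigger a fade-in on the Puddle player character never runs.
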(fn `New Level`
  (`KismetSystemLibrary.PrintString` "bop")
  (bind _output_get (set `self.Level` (+ (`self.Level`) 1)))
  (bind _output_get_2 (set `self.LevelNameArray` (`|MakeArray` (`self.Intro`) (`self.Denial`) (`self.Anger`) (`self.Bargaining`) (`self.Depression`) (`self.Acceptance`))))
  (`GameplayStatics.OpenLevel` (`|GetArrayItem` _output_get_2 _output_get)))