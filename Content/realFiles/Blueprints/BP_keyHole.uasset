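; Clickable keyhole actor for a side-scroller that the player unlocks with a held item.
; Clicking the Cube checks that the player character has the item and that the Box is overlapping a component.
; On success it hides the Cube, disables its collision and sets KeyholeClicked on the character.
; Both outcomes print a debug string.
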(event `self.Cube.OnClicked`
  (params (TouchedComponent :type "PrimitiveComponent Object Reference") (ButtonPressed :type "Key Structure"))
  (bind _cube (`self.Cube`))
  (bind _as2dside_scroller_character (cast `/Game/realFiles/Blueprints/2DSideScrollerCharacter` (`GameplayStatics.GetPlayerPawn` 0)))
  (if (and (`/Game/realFiles/Blueprints/2DSideScrollerCharacter.bDoesHaveItem` _as2dside_scroller_character) (`PrimitiveComponent.IsOverlappingComponent` (`self.Box`) null))
    (`KismetSystemLibrary.PrintString` "you're very cool and good" true true (struct :`R` 1.0 :`A` 1.0))
    (`SceneComponent.SetVisibility` _cube false false)
    (`PrimitiveComponent.SetCollisionEnabled` _cube "NoCollision")
    (bind _as2dside_scroller_character_2 (cast `/Game/realFiles/Blueprints/2DSideScrollerCharacter` (`GameplayStatics.GetPlayerPawn` 0)))
    (set `/Game/realFiles/Blueprints/2DSideScrollerCharacter.bKeyholeClicked` true _as2dside_scroller_character_2)
    (else
      (`KismetSystemLibrary.PrintString` "never try ever again you are bad" true true (struct :`B` 1.0 :`A` 1.0)))))

(fn `UserConstructionScript`)